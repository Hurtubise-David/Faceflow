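; FaceFlowBP is an actor Blueprint that polls a JSON file of keypoints, apparently for face tracking, as a debug readout.
; Every Tick it calls ReadJsonFile on JsonFileName and prints only the call's return value.
; An unconnected chain that would print the parsed server string, server items and item values never runs, and nothing applies the data.
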(event EventBeginPlay)

(event Collision|EventActorBeginOverlap
  (params (OtherActor :type Actor%20Object%20Reference)))

(event EventTick
  (params (DeltaSeconds :type Float%20%28single-precision%29))
  ;[1 1 1] Read KeyPoints
  (bind (_server _serveritems _itemvalue _returnvalue) (Class|JsonPluginBPLibrary|ReadJsonFile (Variables|Default|GetJsonFileName)))
  (Development|PrintString (Utilities|String|ToString(Boolean) _returnvalue)))

(fn ConstructionScript)